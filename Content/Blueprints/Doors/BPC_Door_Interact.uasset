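; Interactive door Blueprint that the player opens and closes with the Interact input while standing near it.
; A Box overlap by the player character enables input and reveals two text renders, and leaving disables input and hides them.
; A FlipFlop on each press alternates between OpenDoor and CloseDoor, which are called here but defined outside this file.
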(event `InputAction|Interact`
  (params (Key :type "Key Structure"))
  (:`Pressed`
    (`/Engine/EditorBlueprintResources/StandardMacros.FlipFlop`
      (:`A`
        (`self.OpenDoor`))
      (:`B`
        (`self.CloseDoor`)))))

(event `self.Box.OnComponentBeginOverlap`
  (params (OverlappedComponent :type "PrimitiveComponent Object Reference") (OtherActor :type "Actor Object Reference") (OtherComp :type "PrimitiveComponent Object Reference") (OtherBodyIndex :type Integer) (bFromSweep :type Boolean) (SweepResult :type "HitResult Structure (by ref)"))
  ;[1 1 1] Overlap - Open/Close Door
  (if (== OtherActor (`GameplayStatics.GetPlayerCharacter` 0))
    (`self.EnableInput` (`GameplayStatics.GetPlayerController` 0))
    (`SceneComponent.SetHiddenInGame` (`self.TextRender1`) false false)
    (`SceneComponent.SetHiddenInGame` (`self.TextRender2`) false false)))

(event `self.Box.OnComponentEndOverlap`
  (params (OverlappedComponent :type "PrimitiveComponent Object Reference") (OtherActor :type "Actor Object Reference") (OtherComp :type "PrimitiveComponent Object Reference") (OtherBodyIndex :type Integer))
  ;[1 1 1] Overlap - Open/Close Door
  (if (== OtherActor (`GameplayStatics.GetPlayerCharacter` 0))
    (`self.DisableInput` (`GameplayStatics.GetPlayerController` 0))
    (`SceneComponent.SetHiddenInGame` (`self.TextRender2`) true false)
    (`SceneComponent.SetHiddenInGame` (`self.TextRender1`) true false)))

(fn `UserConstructionScript`
  (`parent.UserConstructionScript`))