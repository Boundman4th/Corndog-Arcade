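; BP_Door is a key-locked door that opens when an interacting player holds the key for its KeyChannel.
; OnInteraction checks the player with HasKey, then calls Open, which sets IsOpen.
; Open plays the LiftDoor timeline, whose Update triggers the RotateDoor timeline.
; RotateDoor's Update applies both outputs to the Cube component as relative Z location and roll, so the door lifts and rotates.
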(event `/Game/Blueprints/Keys/InteractInterface.OnInteraction`
  (params (Player :type "/Game/SideScrollerBP/Blueprints/SideScrollerCharacter Object Reference"))
  (`/Engine/EditorBlueprintResources/StandardMacros.IsValid` Player
    (:`Is Valid`
      (bind _returnvalue (`/Game/SideScrollerBP/Blueprints/SideScrollerCharacter.HasKey?` Player (`self.KeyChannel`)))
      (if _returnvalue
        (`self.Open`)))))

(event `Open`
  (set `self.IsOpen?` true)
  (bind (_direction _lift_door) (`Timeline|Lift Door`)
    (:`Update`
      (bind (_direction_2 _newtrack_0) (`Timeline|RotateDoor`)
        (:`Update`
          (`SceneComponent.K2_SetRelativeLocationAndRotation` (`self.Cube`) (`KismetMathLibrary.MakeVector` 0.0 0.0 _lift_door) (`KismetMathLibrary.MakeRotator` _newtrack_0) false false))))))

(fn `UserConstructionScript`)